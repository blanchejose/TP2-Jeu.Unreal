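; BP_Chest is a one-time openable chest that credits the interacting player with a collected chest.
; Character overlap shows a text prompt while the chest is closed and hides it on leaving.
; Interact marks it opened, hides the prompt and calls AddChest on the instigator's PS_Collector player state.
; If that cast succeeds, a timeline then swings the lid pivot open by lerping its relative rotation.
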(event `self.ReceiveActorBeginOverlap`
  (params (OtherActor :type "Actor Object Reference"))
  (cast `Character` OtherActor)
  (if (not (`self.bIsOpened`))
    (`SceneComponent.SetVisibility` (`self.PromptText`) true false)))

(event `self.ReceiveActorEndOverlap`
  (params (OtherActor :type "Actor Object Reference"))
  (cast `Character` OtherActor)
  (`SceneComponent.SetVisibility` (`self.PromptText`) false false))

(event `/Game/TP2/Blueprints/BPI_Interactable.Interact`
  (params (InstigatorPawn :type "Pawn Object Reference"))
  (if (not (`self.bIsOpened`))
    (set `self.bIsOpened` true)
    (`SceneComponent.SetVisibility` (`self.PromptText`) false false)
    (bind _asps_collector (cast `/Game/TP2/Blueprints/PS_Collector` (`Pawn.PlayerState` InstigatorPawn)))
    (`/Game/TP2/Blueprints/PS_Collector.AddChest` _asps_collector)
    (bind (_direction _alpha) (`Timeline|TL_OpenLid` :!via `PlayFromStart`)
      (:`Update`
        (`SceneComponent.K2_SetRelativeRotation` (`self.LidPivot`) (`KismetMathLibrary.RLerp` (struct) (struct :`Pitch` 80.0) _alpha) false false)))))

(fn `UserConstructionScript`)